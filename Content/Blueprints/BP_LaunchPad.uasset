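; BP_LaunchPad is a launch pad that tilts open and swings back when its Launch event is called.
; Launch calls MoveLaunchPad, waits half a second, then calls it again, with a FlipFlop alternating between playing the timeline and reversing it from the end.
; The timeline lerps the spring arm component's relative pitch from zero to OpenAngle, using it as the pad's pivot.
; The graph itself applies no force to other actors.
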(event EventBeginPlay)

(event Collision|EventActorBeginOverlap
  (params (OtherActor :type Actor%20Object%20Reference)))

(event EventTick
  (params (DeltaSeconds :type Float%20%28single-precision%29)))

(event EventLaunch
  (Class|RPLaunchPad|MoveLaunchPad)
  (Utilities|FlowControl|Delay 0.5)
  (Class|RPLaunchPad|MoveLaunchPad))

(event EventMoveLaunchPad
  (Utilities|FlowControl|FlipFlop
    (:A
      ;[1 1 1] Rotate LaunchPad
      (bind _startlaunch (Timeline|Launch Play)
        (:Update
          (Transformation|SetRelativeRotation (Variables|Default|GetSpringArmComponent) (Math|Rotator|MakeRotator 0.0 (Math|Float|Lerp 0.0 (Variables|Default|GetOpenAngle) _startlaunch) 0.0) false false))))
    (:B
      (Timeline|Launch ReverseFromEnd))))

(fn ConstructionScript)